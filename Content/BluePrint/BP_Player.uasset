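; Player character Blueprint with camera-relative movement, a sprint with timeline-driven forward dash, and a melee combo attack.
; An IDLE/BATTLE state, mapped to IsIdle every Tick, blocks movement input and sprint during attacks.
; Left click starts an attack with a forward sphere trace or buffers the next hit, which NextAttackCheck_Event fires.
; OnAnimEndCheck_Event resets the combo to idle; Right Shift sets a fixed world-X velocity.
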(event `Key|RightShift`
  (params (Key :type "Key Structure"))
  (:`Pressed`
    (set `MovementComponent.Velocity` (5000.0 0.0 0.0) (`self.CharacterMovement`))))

(event `InputAxis|MoveForward` :overrideparent false
  (params (AxisValue :type "Float (single-precision)"))
  (if (`self.IsIdle`)
    (`self.AddMovementInput` (`KismetMathLibrary.GetForwardVector` (`KismetMathLibrary.MakeRotator` 0.0 0.0 (.yaw (`self.GetControlRotation`)))) AxisValue)))

(event `Key|LeftShift`
  (params (Key :type "Key Structure"))
  (bind _charactermovement (`self.CharacterMovement`))
  (:`Pressed`
    (if (`self.IsIdle`)
      (set `CharacterMovementComponent.MaxWalkSpeed` 600.0 _charactermovement)
      (bind (_direction `_새_트랙_0`) (`Timeline|타임라인_0` :!via `PlayFromStart`)
        (:`Update`
          (`self.K2_SetActorLocation` (+ (* (`KismetMathLibrary.GetForwardVector` (`self.K2_GetActorRotation`)) `_새_트랙_0`) (`self.K2_GetActorLocation`)))))))
  (:`Released`
    (if (`self.IsIdle`)
      (set `CharacterMovementComponent.MaxWalkSpeed` 275.0 _charactermovement))))

(event `InputAxis|MoveRight` :overrideparent false
  (params (AxisValue :type "Float (single-precision)"))
  (if (`self.IsIdle`)
    (`self.AddMovementInput` (`KismetMathLibrary.GetRightVector` (`KismetMathLibrary.MakeRotator` 0.0 0.0 (.yaw (`self.GetControlRotation`)))) AxisValue)))

(event `Key|LeftMouseButton`
  (params (Key :type "Key Structure"))
  (bind _returnvalue (`self.K2_GetActorLocation`))
  (:`Pressed`
    (if (`self.IsAttack`)
      (set `self.IsNextCombo` true)
      (else
        (set `self.IsAttack` true)
        (set `self.CurrentStatePawn` "NewEnumerator1")
        (`KismetSystemLibrary.SphereTraceSingleForObjects` :`Start` _returnvalue :`End` (+ _returnvalue (* (`SceneComponent.GetForwardVector` (`self.CapsuleComponent`)) 150.0)) :`Radius` 30.0 :`ObjectTypes` (`|MakeArray` "ObjectTypeQuery8" :!type "EObjectTypeQuery Enum") :`DrawDebugType` "ForDuration" :!label _label)))))

(event `InputAxis|Turn` :overrideparent false
  (params (AxisValue :type "Float (single-precision)"))
  (`self.AddControllerYawInput` AxisValue))

(event `InputAxis|LookUp` :overrideparent false
  (params (AxisValue :type "Float (single-precision)"))
  (`self.AddControllerPitchInput` AxisValue))

(event `NextAttackCheck_Event`
  (if (`self.IsNextCombo`)
    (set `self.IsNextCombo` false)
    (bind _output_get (set `self.ComboCount` (+ (`self.ComboCount`) 1)))
    (switch `int` _output_get
      (:`1`
        (goto _label))
      (:`2`
        (goto _label)))))

(event `self.ReceiveTick`
  (params (DeltaSeconds :type "Float (single-precision)"))
  (switch `/Game/BluePrint/BPE_PlayerState` (`self.CurrentStatePawn`)
    (:`NewEnumerator0`
      (set `self.IsIdle` true))
    (:`NewEnumerator1`
      (set `self.IsIdle` false))))

(event `OnAnimEndCheck_Event`
  (set `self.IsAttack` false)
  (set `self.ComboCount` 0)
  (set `self.IsNextCombo` false)
  (set `self.CurrentStatePawn` "NewEnumerator0"))

(fn `NextAttack`
  (returns (bNextAttack :type Boolean))
  (if (`self.IsNextCombo`)
    (bind _output_get (set `self.IsNextCombo` false))
    (set `self.ComboCount` (+ (`self.ComboCount`) 1))
    (return _output_get)))

(fn `UserConstructionScript`)